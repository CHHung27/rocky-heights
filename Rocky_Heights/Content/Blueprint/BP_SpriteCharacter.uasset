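; BP_SpriteCharacter is a side-scrolling 2D player character with a flipbook sprite.
; The MoveRight input axis moves it along the world X axis.
; Each Tick picks the run or idle flipbook, depending on whether movement velocity is above zero.
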(event Custom|updateanimation
  (Sprite|SetFlipbook (Variables|Default|GetSprite) (select (> (Math|Vector|VectorLength (Variables|/Script/Engine.MovementComponent|GetVelocity (Variables|Character|GetCharacterMovement))) 0.0) "/Game/Assets/sprites/player/run/FB_Player_Run.FB_Player_Run" "/Game/Assets/sprites/player/idle/FB_Payer_Idle.FB_Payer_Idle")))

(event EventTick
  (params (DeltaSeconds :type Float%20%28single-precision%29))
  (CallFunction|Updateanimation))

(event Input|AxisEvents|InputAxisMoveRight
  (params (AxisValue :type Float%20%28single-precision%29))
  (Pawn|Input|AddMovementInput "1.000000,0.000000,0.000000" AxisValue false))

(fn ConstructionScript)